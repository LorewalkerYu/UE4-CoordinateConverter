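; BP_CoodinateConverter_Test is a test actor for the SqureConverter coordinate converter.
; On BeginPlay it constructs the converter and initializes it with two corners, each pairing string coordinates with a 2D point.
; It then converts a hard-coded negative coordinate far outside that square.
; If conversion succeeds, it spawns a movable cube StaticMeshActor at the resulting X/Y location.
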(event EventBeginPlay
  (bind _returnvalue (Game|ConstructObjectfromClass "/Script/CoordinateConverter.SqureConverter" self))
  (bind _output_get (Variables|Default|SetSqureConverter _returnvalue))
  (bind _returnvalue_2 (Class|SqureConverter|Init _output_get "0" "0" (Math|Vector2D|MakeVector2D 0.0 0.0) "10" "10" (Math|Vector2D|MakeVector2D 1e+02 1e+02)))
  (if _returnvalue_2
    (bind (_outlocation _returnvalue_3) (Class|SqureConverter|ConvertPointtoLocation (Variables|Default|GetSqureConverter) "-12121" "-1123124"))
    (if _returnvalue_3
      (bind _returnvalue_4 (Game|SpawnActorfromClass "/Script/Engine.StaticMeshActor" (Math|Transform|MakeTransform (Math|Vector|MakeVector (.x _outlocation) (.y _outlocation) 0.0) "0, 0, 0" "1,1,1") "AlwaysSpawn" 0 0))
      (Transformation|SetMobility _returnvalue_4 "Movable")
      (Components|StaticMesh|SetStaticMesh (Variables|/Script/Engine.StaticMeshActor|GetStaticMeshComponent _returnvalue_4) "/Game/WaiBuDaoRu/Geometry/Meshes/1M_Cube.1M_Cube"))))

(event Collision|EventActorBeginOverlap
  (params (OtherActor :type Actor%20Object%20Reference)))

(event EventTick
  (params (DeltaSeconds :type Float%20%28single-precision%29)))

(fn ConstructionScript)