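; Coordinate converter Blueprint that holds a SqureConverter object for mapping longitude/latitude strings to world X/Y locations.
; BeginPlay constructs the converter and calls Init with two opposite corners, top-left and bottom-right, each pairing geographic coordinates with a 2D world point.
; An unwired test backup uses different corners, converts six sample points and spawns tall static mesh actor markers, printing a message on failure.
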(event EventBeginPlay
  (bind _returnvalue (Game|ConstructObjectfromClass "/Script/CoordinateConverter.SqureConverter" self))
  (Variables|Default|SetSqureConverter _returnvalue)
  (Class|SqureConverter|Init (Variables|Default|GetSqureConverter) "114.840817" "38.289736" (Math|Vector2D|MakeVector2D 154.313477 -1340.87561) "122.717304" "34.376268" (Math|Vector2D|MakeVector2D 2138.891602 -135.01355)))

(fn ConstructionScript)